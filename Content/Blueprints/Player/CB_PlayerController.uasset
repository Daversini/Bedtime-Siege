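; Player controller that handles grid-snapped tower placement with the mouse, entering placement mode on BeginPlay.
; Enabling the mode spawns a preview of PlaceableActorType far below the world, flags its clickable component and adds a ploppable component.
; Each tick, a cursor line trace moves the preview to the GridManager's closest grid position.
; Left-click spawns the tower if the ploppable component reports valid placement, then exits the mode, destroying the preview.
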(event `self.ReceiveBeginPlay`
  (`self.SetPlacementModeEnabled` true))

(event `self.ReceiveTick`
  (params (DeltaSeconds :type "Float (single-precision)"))
  (if (`self.PlacementModeEnabled`)
    (`self.UpdatePlacement`)))

(event `InputAction|MouseLeftClick`
  (params (Key :type "Key Structure"))
  (:`Pressed`
    (if (`self.PlacementModeEnabled`)
      (`self.SpawnTower`))))

(fn `SetPlacementModeEnabled`
  (params (IsEnabled :type Boolean))
  (bind _placeableactor (`self.PlaceableActor`))
  (if (== IsEnabled (`self.PlacementModeEnabled`))
    (return)
    (else
      (bind _output_get (set `self.PlacementModeEnabled` IsEnabled))
      (if _output_get
        (bind _returnvalue (`|SpawnActorFromClass` (`self.PlaceableActorType`) (`KismetMathLibrary.MakeTransform` (0.0 0.0 -100000.0)) "AlwaysSpawn" "OverrideRootScale" null null))
        (bind _output_get_2 (set `self.PlaceableActor` _returnvalue))
        (bind _returnvalue_2 (`self.GetComponentByClass` _output_get_2 "/Game/Blueprints/GameObjects/Components/CB_ClickableComponent.CB_ClickableComponent_C"))
        (`/Engine/EditorBlueprintResources/StandardMacros.IsValid` _returnvalue_2
          (:`Is Valid`
            (`/Game/Blueprints/GameObjects/Components/CB_ClickableComponent.InPlacementMode` _returnvalue_2))
          (:`Is Not Valid`
            _))
        (`AddComponent|NODE_AddCB_PloppableComponent-0` :`self` _output_get_2)
        (else
          (`/Engine/EditorBlueprintResources/StandardMacros.IsValid` _placeableactor
            (:`Is Valid`
              (`self.K2_DestroyActor` _placeableactor))))))))

(fn `SpawnTower`
  (bind _returnvalue (`self.GetComponentByClass` (`self.PlaceableActor`) "/Game/Blueprints/GameObjects/Components/CB_PloppableComponent.CB_PloppableComponent_C"))
  (`/Engine/EditorBlueprintResources/StandardMacros.IsValid` _returnvalue
    (:`Is Valid`
      (if (`/Game/Blueprints/GameObjects/Components/CB_PloppableComponent.isPlacementValid` _returnvalue)
        (`|SpawnActorFromClass` (`self.PlaceableActorType`) (`self.GetTransform` (`self.PlaceableActor`)) "AlwaysSpawn" "OverrideRootScale" null null)
        (`self.SetPlacementModeEnabled` false)))))

(fn `UpdatePlacement`
  (bind (_worldlocation _worlddirection) (`self.DeprojectMousePositionToWorld`))
  (bind _outhit (`KismetSystemLibrary.LineTraceSingle` _worldlocation (+ _worlddirection (* _worlddirection 10000.0)) "TraceTypeQuery3"))
  (bind (_bblockinghit _binitialoverlap _time _distance _location) (`GameplayStatics.BreakHitResult` _outhit))
  (if _bblockinghit
    (bind _returnvalue (`GameplayStatics.GetActorOfClass` "/Game/Blueprints/Grid/GridManager.GridManager_C"))
    (bind _outputvector (`/Game/Blueprints/Grid/GridManager.GetClosestGridPosition` _returnvalue _location))
    (`self.K2_SetActorLocation` (`self.PlaceableActor`) _outputvector false false)))

(fn `UserConstructionScript`)